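; DamagePack is a hazard actor that damages the player on contact and then destroys itself.
; When its Cube is hit by a BP_Player, it subtracts a fixed amount of Health, prints a message and destroys the actor.
; If Health equals exactly zero, it flags the player dead and shows the restart display.
; The FIRE input enters the same print, destroy and death-check chain without applying damage.
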(event OnComponentHit(Cube)
  (params (HitComponent :type Primitive%20Component%20Object%20Reference) (OtherActor :type Actor%20Object%20Reference) (OtherComp :type Primitive%20Component%20Object%20Reference) (NormalImpulse :type Vector :default "0, 0, 0") (Hit :type Hit%20Result%20Structure%20%28by%20ref%29))
  (Variables|Default|SetTags (Utilities|Array|MakeArray "DamagePack"))
  (bind _asbp_player (Utilities|Casting|CastToBP_Player OtherActor))
  (Variables|/Game/InfiniteMatrix/Blueprints/BP_Player.BP_Player_C|SetHealth _asbp_player (- (Variables|/Game/InfiniteMatrix/Blueprints/BP_Player.BP_Player_C|GetHealth _asbp_player) 0.25))
  (Development|PrintString "-.025 health!")
  (Actor|DestroyActor)
  (if (== (Variables|/Game/InfiniteMatrix/Blueprints/BP_Player.BP_Player_C|GetHealth _asbp_player) 0.0)
    (Variables|/Game/InfiniteMatrix/Blueprints/BP_Player.BP_Player_C|SetIsDead _asbp_player true)
    (Default|DisplayRestart _asbp_player)))

(event EventBeginPlay)

(event Collision|EventActorBeginOverlap
  (params (OtherActor :type Actor%20Object%20Reference)))

(event EventTick
  (params (DeltaSeconds :type Float%20%28single-precision%29)))

(event Input|ActionEvents|InputActionFIRE
  (params (Key :type Key%20Structure :default "None"))
  (:Pressed
    (Development|PrintString "-.025 health!")
    (Actor|DestroyActor)
    (if (== (Variables|/Game/InfiniteMatrix/Blueprints/BP_Player.BP_Player_C|GetHealth (stale OnComponentHit(Cube) _asbp_player)) 0.0)
      (Variables|/Game/InfiniteMatrix/Blueprints/BP_Player.BP_Player_C|SetIsDead (stale OnComponentHit(Cube) _asbp_player) true)
      (Default|DisplayRestart (stale OnComponentHit(Cube) _asbp_player)))))

(fn ConstructionScript)