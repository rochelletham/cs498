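; BP_TunnelSpawner is an unfinished spawner for BP_Tunnel segments, apparently meant to chain them end to end.
; SpawnTunnel spawns a tunnel at a given location and stores it as NewestTunnel.
; Unwired calls would place the next tunnel at NewestTunnel's root or SpawnPoint location.
; Nothing in this Blueprint triggers spawning: SpawnTunnelAtSpawnPoint is empty, and the event graph has no active logic.
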(event Collision|EventActorBeginOverlap
  (params (OtherActor :type Actor%20Object%20Reference)))

(event EventTick
  (params (DeltaSeconds :type Float%20%28single-precision%29)))

(fn ConstructionScript)

(fn SpawnTunnel
  (params (SpawnLocation :type Vector))
  (bind _returnvalue (Game|SpawnActorfromClass "/Game/InfiniteMatrix/Blueprints/BP_Tunnel.BP_Tunnel_C" (Math|Transform|MakeTransform SpawnLocation "0, 0, 0" "1,1,1") "Undefined" 0 0))
  (Variables|Default|SetNewestTunnel _returnvalue))

(fn SpawnTunnelatSpawnPoint)